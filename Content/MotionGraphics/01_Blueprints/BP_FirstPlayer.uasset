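; First player pawn: a physics-driven mesh moved by camera-relative forces, which also relays input for a second player.
; On BeginPlay it adds the input mapping context and finds BP_SecondPlayer, forwarding that player's move values and zeroing them on release.
; Hits on floor-tagged actors arm a single force-based jump.
; The wall-tag branch is empty, and its Niagara wall-touch effect is left disconnected.
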(event `self.ReceiveBeginPlay`
  (bind _asplayer_controller (cast `PlayerController` (`self.GetController`)))
  (message `EnhancedInputSubsystemInterface.AddMappingContext` (pcsubsystem `EnhancedInputLocalPlayerSubsystem` _asplayer_controller) "/Game/MotionGraphics/10_Misc/Inputs/IMC_Player.IMC_Player" 0 (struct))
  (bind _returnvalue (`GameplayStatics.GetActorOfClass` "/Game/MotionGraphics/01_Blueprints/BP_SecondPlayer.BP_SecondPlayer_C"))
  (set `self.SecondPlayer` _returnvalue))

(event `EnhancedInput|/Game/MotionGraphics/10_Misc/Inputs/IA_MoveRight_Second`
  (params (ActionValue :type "Float (double-precision)") (ElapsedSeconds :type "Float (double-precision)") (TriggeredSeconds :type "Float (double-precision)") (InputAction :type "InputAction Object Reference" :default "/Game/MotionGraphics/10_Misc/Inputs/IA_MoveRight_Second.IA_MoveRight_Second"))
  (bind _secondplayer (`self.SecondPlayer`))
  (:`Triggered`
    (`/Engine/EditorBlueprintResources/StandardMacros.IsValid` _secondplayer
      (:`Is Valid`
        (`/Game/MotionGraphics/01_Blueprints/BP_SecondPlayer.UpdateRightValue` _secondplayer ActionValue))))
  (:`Completed`
    (`/Engine/EditorBlueprintResources/StandardMacros.IsValid` _secondplayer
      (:`Is Valid`
        (`/Game/MotionGraphics/01_Blueprints/BP_SecondPlayer.UpdateRightValue` _secondplayer 0.0)))))

(event `EnhancedInput|/Game/MotionGraphics/10_Misc/Inputs/IA_MoveUp`
  (params (ActionValue :type "Float (double-precision)") (ElapsedSeconds :type "Float (double-precision)") (TriggeredSeconds :type "Float (double-precision)") (InputAction :type "InputAction Object Reference" :default "/Game/MotionGraphics/10_Misc/Inputs/IA_MoveUp.IA_MoveUp"))
  (bind (_returnvalue_x _returnvalue_y) (`KismetMathLibrary.BreakVector` (`KismetMathLibrary.GetForwardVector` (`PlayerCameraManager.GetCameraRotation` (`GameplayStatics.GetPlayerCameraManager` 0)))))
  ;[1 1 1] First Player Input
  (:`Triggered`
    (`PrimitiveComponent.AddForce` (`self.StaticMesh`) (* ActionValue (`KismetMathLibrary.MakeVector` _returnvalue_x _returnvalue_y) (`self.Horizontal Force`)) "None" false)))

(event `EnhancedInput|/Game/MotionGraphics/10_Misc/Inputs/IA_MoveUp_Second`
  (params (ActionValue :type "Float (double-precision)") (ElapsedSeconds :type "Float (double-precision)") (TriggeredSeconds :type "Float (double-precision)") (InputAction :type "InputAction Object Reference" :default "/Game/MotionGraphics/10_Misc/Inputs/IA_MoveUp_Second.IA_MoveUp_Second"))
  (bind _secondplayer (`self.SecondPlayer`))
  (:`Triggered`
    (`/Engine/EditorBlueprintResources/StandardMacros.IsValid` _secondplayer
      (:`Is Valid`
        (`/Game/MotionGraphics/01_Blueprints/BP_SecondPlayer.UpdateUpValue` _secondplayer ActionValue))))
  (:`Completed`
    (`/Engine/EditorBlueprintResources/StandardMacros.IsValid` _secondplayer
      (:`Is Valid`
        (`/Game/MotionGraphics/01_Blueprints/BP_SecondPlayer.UpdateUpValue` _secondplayer 0.0)))))

(event `EnhancedInput|/Game/MotionGraphics/10_Misc/Inputs/IA_MoveRight`
  (params (ActionValue :type "Float (double-precision)") (ElapsedSeconds :type "Float (double-precision)") (TriggeredSeconds :type "Float (double-precision)") (InputAction :type "InputAction Object Reference" :default "/Game/MotionGraphics/10_Misc/Inputs/IA_MoveRight.IA_MoveRight"))
  (bind (_returnvalue_x _returnvalue_y) (`KismetMathLibrary.BreakVector` (`KismetMathLibrary.GetRightVector` (`PlayerCameraManager.GetCameraRotation` (`GameplayStatics.GetPlayerCameraManager` 0)))))
  ;[1 1 1] First Player Input
  (:`Triggered`
    (`PrimitiveComponent.AddForce` (`self.StaticMesh`) (* ActionValue (`KismetMathLibrary.MakeVector` _returnvalue_x _returnvalue_y) (`self.Horizontal Force`)) "None" false)))

(event `EnhancedInput|/Game/MotionGraphics/10_Misc/Inputs/IA_Jump`
  (params (ActionValue :type "Float (double-precision)") (ElapsedSeconds :type "Float (double-precision)") (TriggeredSeconds :type "Float (double-precision)") (InputAction :type "InputAction Object Reference" :default "/Game/MotionGraphics/10_Misc/Inputs/IA_Jump.IA_Jump"))
  ;[1 1 1] First Player Input
  (:`Triggered`
    (`/Engine/EditorBlueprintResources/StandardMacros.IsValid` (`self.FloorCollider`)
      (:`Is Valid`
        (set `self.FloorCollider` null)
        (`PrimitiveComponent.AddForce` (`self.StaticMesh`) (* (0.0 0.0 1.0) (`self.Jump Force`)) "None" false)))))

(event `self.StaticMesh.OnComponentHit`
  (params (HitComponent :type "PrimitiveComponent Object Reference") (OtherActor :type "Actor Object Reference") (OtherComp :type "PrimitiveComponent Object Reference") (NormalImpulse :type "Vector Structure") (Hit :type "HitResult Structure (by ref)"))
  (`|ExecutionSequence`
    (:`then_0`
      (if (`self.ActorHasTag` OtherActor "tag_floor")
        (set `self.FloorCollider` OtherActor)))
    (:`then_1`
      (if (`self.ActorHasTag` OtherActor "tag_wall")
        _))))

(fn `UserConstructionScript`)