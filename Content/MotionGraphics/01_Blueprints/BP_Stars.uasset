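; BP_Stars is a collectible star goal that completes a quest when an actor tagged as the player touches it.
; On overlap, the Expand timeline scales the mesh to double size, then spawns a Niagara burst and hides the mesh with collision off.
; After a short delay, GoalAchived runs the parent logic, notifies BP_GameMode_Base that the quest finished, and the actor destroys itself.
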(event `self.GoalAchived`
  (`parent.GoalAchived`)
  (bind _asbp_game_mode_base (cast `/Game/MotionGraphics/01_Blueprints/BP_GameMode_Base` (`GameplayStatics.GetGameMode`)))
  (`/Game/MotionGraphics/01_Blueprints/BP_GameMode_Base.QuestFinished` _asbp_game_mode_base))

(event `self.StaticMesh.OnComponentBeginOverlap`
  (params (OverlappedComponent :type "PrimitiveComponent Object Reference") (OtherActor :type "Actor Object Reference") (OtherComp :type "PrimitiveComponent Object Reference") (OtherBodyIndex :type Integer) (bFromSweep :type Boolean) (SweepResult :type "HitResult Structure (by ref)"))
  (bind _staticmesh (`self.StaticMesh`))
  (if (`self.ActorHasTag` OtherActor "tag_player")
    (bind (_direction _ratio) (`Timeline|Expand`)
      (:`Update`
        (`SceneComponent.SetWorldScale3D` (`self.StaticMesh`) (`KismetMathLibrary.VLerp` (1.0 1.0 1.0) (2.0 2.0 2.0) _ratio)))
      (:`Finished`
        (`NiagaraFunctionLibrary.SpawnSystemAtLocation` "/Game/MotionGraphics/04_VFX/NS_Star_Explode.NS_Star_Explode" (`SceneComponent.K2_GetComponentLocation` _staticmesh))
        (`SceneComponent.SetHiddenInGame` _staticmesh true false)
        (`PrimitiveComponent.SetCollisionEnabled` _staticmesh "NoCollision")
        (`KismetSystemLibrary.Delay` 1.0)
        (`self.GoalAchived`)
        (`self.K2_DestroyActor`)))))

(fn `UserConstructionScript`)