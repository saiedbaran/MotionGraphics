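; BP_CylinderArrow is a motion-graphics arrow that turns, moves vertically and changes color in response to a target actor.
; CalculateRelativeZ remaps target distance through a power and float curve to get a height, plus a horizontal look-at rotation.
; While enabled by ToggleUpdateTransform, Tick eases the mesh's relative Z with a fixed-step FInterpTo, sets rotation directly and drives a dynamic material's color_ratio from the curve value.
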(event `self.ReceiveBeginPlay`
  (bind _cylinderarrow (`self.CylinderArrow`))
  (bind _returnvalue (`PrimitiveComponent.CreateDynamicMaterialInstance` _cylinderarrow 0 (`PrimitiveComponent.GetMaterial` _cylinderarrow 0) "None"))
  (set `self.Cylinder Dynamic Material` _returnvalue))

(event `self.ReceiveTick`
  (params (DeltaSeconds :type "Float (single-precision)"))
  (bind (_relative_z _ratio _relativerotation _curvevalue) (`self.CalculateRelativeZ`))
  (bind _cylinderarrow (`self.CylinderArrow`))
  (bind (_relativelocation_x _relativelocation_y _relativelocation_z) (`KismetMathLibrary.BreakVector` (`SceneComponent.RelativeLocation` (`self.CylinderArrow`))))
  (if (`self.isUpdatingTransform`)
    (`SceneComponent.K2_SetRelativeLocation` _cylinderarrow (`KismetMathLibrary.MakeVector` 0.0 0.0 (`KismetMathLibrary.FInterpTo` _relativelocation_z _relative_z 0.5 0.5)) false false)
    (`SceneComponent.K2_SetRelativeRotation` _cylinderarrow _relativerotation false false)
    (`MaterialInstanceDynamic.SetScalarParameterValue` (`self.Cylinder Dynamic Material`) "color_ratio" (`KismetMathLibrary.MultiplyMultiply_FloatFloat` _curvevalue (`self.BaseColorPower`)))))

(event `ToggleUpdateTransform`
  (params (isActive :type Boolean))
  (set `self.isUpdatingTransform` isActive))

(fn `CalculateRelativeZ`
  (returns (`Relative Z` :type "Float (double-precision)") (ratio :type "Float (double-precision)") (RelativeRotation :type "Rotator Structure") (CurveValue :type "Float (double-precision)"))
  (bind (_returnvalue_x _returnvalue_y) (`KismetMathLibrary.BreakVector` (`self.K2_GetActorLocation`)))
  (bind (_returnvalue_x_2 _returnvalue_y_2) (`KismetMathLibrary.BreakVector` (`self.K2_GetActorLocation` (`self.TargetActor`))))
  (bind _returnvalue (`KismetMathLibrary.MapRangeClamped` (`KismetMathLibrary.Vector_Distance` (`self.K2_GetActorLocation`) (`self.K2_GetActorLocation` (`self.TargetActor`))) (`self.Minimum Distance`) (`self.Maximum Distance`) 0.0 1.0))
  (bind _returnvalue_2 (`CurveFloat.GetFloatValue` (`self.LerpCurve`) (`KismetMathLibrary.MultiplyMultiply_FloatFloat` _returnvalue (`self.CurvePower`))))
  (return (`KismetMathLibrary.Lerp` -18.0 -0.5 _returnvalue_2) _returnvalue (`KismetMathLibrary.FindLookAtRotation` (`KismetMathLibrary.MakeVector` _returnvalue_x _returnvalue_y) (`KismetMathLibrary.MakeVector` _returnvalue_x_2 _returnvalue_y_2)) _returnvalue_2))

(fn `UserConstructionScript`)