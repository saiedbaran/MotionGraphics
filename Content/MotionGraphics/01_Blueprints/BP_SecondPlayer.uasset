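; Second-player Blueprint: a mesh character steered on the world XY plane that explodes and respawns when it hits a floor-tagged actor.
; BeginPlay enables player-two input and adds its mapping context, though the move-up action only prints debug text.
; Externally callable update events store axis values, which Tick converts into mesh rotation and unswept offsets.
; Floor hits hide the mesh, spawn Niagara, then after a delay request respawn from BP_GameMode_Base and destroy the actor.
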(event `self.ReceiveBeginPlay`
  (`self.EnableInput` (`GameplayStatics.GetPlayerController` 1))
  (bind _asplayer_controller (cast `PlayerController` (`self.GetController`)))
  (`EnhancedInputSubsystemInterface.AddMappingContext` (pcsubsystem `EnhancedInputLocalPlayerSubsystem` _asplayer_controller) "/Game/MotionGraphics/10_Misc/Inputs/IMC_SecondPlayer.IMC_SecondPlayer" 0 (struct)))

(event `self.ReceiveTick`
  (params (DeltaSeconds :type "Float (single-precision)"))
  (bind (_direction _speedratio) (`self.GetMovementDirectionAndSpeed`))
  (bind (_direction_2 _speedratio_2) (`self.GetMovementDirectionAndSpeed`))
  (bind _sm_secondcharacter (`self.SM_SecondCharacter`))
  (bind _returnvalue (* (* _direction _speedratio) (`self.MaxSpeed`) DeltaSeconds))
  (if (>= _speedratio_2 0.1)
    (`SceneComponent.K2_SetRelativeRotation` _sm_secondcharacter (`KismetMathLibrary.MakeRotFromX` _direction_2) false false)
    (`KismetSystemLibrary.PrintString` (`KismetStringLibrary.Conv_VectorToString` _returnvalue) true true (struct :`G` 0.66 :`B` 1.0 :`A` 1.0) 0.0)
    (`SceneComponent.K2_AddWorldOffset` (`self.SM_SecondCharacter`) _returnvalue false false)
    (else
      (`SceneComponent.K2_SetRelativeRotation` :`self` _sm_secondcharacter))))

(event `EnhancedInput|/Game/MotionGraphics/10_Misc/Inputs/IA_MoveUp_Second`
  (params (ActionValue :type "Float (double-precision)") (ElapsedSeconds :type "Float (double-precision)") (TriggeredSeconds :type "Float (double-precision)") (InputAction :type "InputAction Object Reference" :default "/Game/MotionGraphics/10_Misc/Inputs/IA_MoveUp_Second.IA_MoveUp_Second"))
  (:`Triggered`
    (`KismetSystemLibrary.PrintString` (`KismetStringLibrary.Concat_StrStr` "Triggered: " (`KismetStringLibrary.Conv_DoubleToString` ActionValue)) true true (struct :`G` 0.66 :`B` 1.0 :`A` 1.0) 0.1))
  (:`Completed`
    (`KismetSystemLibrary.PrintString` "Completed" true true (struct :`R` 1.0 :`B` 0.057309 :`A` 1.0) 5.0)))

(event `UpdateRightValue`
  (params (value :type "Float (double-precision)"))
  ;[1 1 1] Update Value
  (set `self.RightValue` value))

(event `UpdateUpValue`
  (params (value :type "Float (double-precision)"))
  ;[1 1 1] Update Value
  (set `self.UpValue` value))

(event `self.SM_SecondCharacter.OnComponentBeginOverlap`
  (params (OverlappedComponent :type "PrimitiveComponent Object Reference") (OtherActor :type "Actor Object Reference") (OtherComp :type "PrimitiveComponent Object Reference") (OtherBodyIndex :type Integer) (bFromSweep :type Boolean) (SweepResult :type "HitResult Structure (by ref)")))

(event `self.SM_SecondCharacter.OnComponentHit`
  (params (HitComponent :type "PrimitiveComponent Object Reference") (OtherActor :type "Actor Object Reference") (OtherComp :type "PrimitiveComponent Object Reference") (NormalImpulse :type "Vector Structure") (Hit :type "HitResult Structure (by ref)"))
  (if (`self.ActorHasTag` OtherActor "tag_floor")
    (`SceneComponent.SetHiddenInGame` (`self.SM_SecondCharacter`) true false)
    (`NiagaraFunctionLibrary.SpawnSystemAtLocation` "/Game/MotionGraphics/04_VFX/NS_Character_Explode.NS_Character_Explode" (`SceneComponent.K2_GetComponentLocation` (`self.SM_SecondCharacter`)))
    (`KismetSystemLibrary.Delay` 1.0)
    (bind _asbp_game_mode_base (cast `/Game/MotionGraphics/01_Blueprints/BP_GameMode_Base` (`GameplayStatics.GetGameMode`)))
    (`/Game/MotionGraphics/01_Blueprints/BP_GameMode_Base.SpawnSecondPlayer` _asbp_game_mode_base)
    (`self.K2_DestroyActor`)))

(fn `GetMovementDirectionAndSpeed`
  (returns (Direction :type "Vector Structure") (SpeedRatio :type "Float (double-precision)"))
  (bind _returnvalue (+ (* (`self.RightValue`) (`KismetMathLibrary.MakeVector` 0.0 1.0)) (* (`self.UpValue`) (`KismetMathLibrary.MakeVector` -1.0))))
  (return (`KismetMathLibrary.Normal` _returnvalue) (`KismetMathLibrary.FClamp` (`KismetMathLibrary.VSize` _returnvalue))))

(fn `UserConstructionScript`)